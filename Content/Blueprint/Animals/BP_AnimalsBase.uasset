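; BP_AnimalsBase is an animal base Blueprint that configures each animal from category data via GetItemData and DTAnimalCategory.
; The construction script applies that data's mesh and capsule size.
; CheckHungerLevel resets hunger to maximum, subtracts a clamped decrease, then calls CheckHealth, which reloads maximum health before setting the Die flag.
; Thirst, state, enemy and lifetime checks are empty stubs.
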(fn ConstructionScript
  (bind _dt_animalcategory (Variables|Default|GetDT_AnimalCategory))
  (bind _capsule (Variables|Default|GetCapsule))
  (bind _out_row (CallFunction|GetItemData _dt_animalcategory))
  (bind (_name _animaltype _foodtype _hungerdecreaselevel _thirstylevel _maxthirstylevel _maxhelath _mesh _attackeatanimation _attackeathingsound _height _radius) (Utilities|Struct|BreakS_AnimalCategory _out_row))
  (Components|SkeletalMesh|SetSkeletalMeshAsset (Variables|Default|GetSK_Mesh) _mesh)
  (Components|Capsule|SetCapsuleHalfHeight _capsule _height true)
  (Components|Capsule|SetCapsuleRadius _capsule _radius true))

(fn CheckHungerLevel
  (LocalVariables|SetcurrentHungerLvl (LocalVariables|GetmaxHungerLvl))
  (LocalVariables|SetcurrentHungerLvl (Math|Float|Clamp(Float) (- (LocalVariables|GetcurrentHungerLvl) (.HungerDecreaseLevel (Utilities|Struct|BreakS_AnimalCategory (CallFunction|GetItemData (Variables|Default|GetDT_AnimalCategory))))) 0.0 (LocalVariables|GetmaxHungerLvl)))
  (CallFunction|CheckHealth))

(fn CheckHealth
  (LocalVariables|SetcurrentHealth (.MaxHelath (Utilities|Struct|BreakS_AnimalCategory (CallFunction|GetItemData (Variables|Default|GetDT_AnimalCategory)))))
  (if (<= (LocalVariables|GetcurrentHealth) 0.0)
    (Variables|Default|SetbDie true)
    (else
      (Variables|Default|SetbDie false))))

(fn CheckThirstyLevel)

(fn CheckStates)

(fn CheckEnemy)

(fn CheckLifetimeCycle)